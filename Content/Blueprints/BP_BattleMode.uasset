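; BP_BattleMode is a battle game mode that applies a lifesteal heal to the first player's character when a character dies.
; PostLogin binds the death handler, which casts player 0 to CharacterBase without checking who died or killed.
; It builds a GE_HealFromLifesteal spec with the negated product of two attribute reads as a Data.Damage set-by-caller magnitude, then applies it to that player's ability system.
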(event Custom|OncharDied
  (params (Character :type Character%20Base%20Object%20Reference))
  (bind _ascharacter_base (Utilities|Casting|CastToCharacterBase (Game|GetPlayerCharacter 0)))
  (bind _returnvalue (Ability|GameplayEffect|AssignTagSetbyCallerMagnitude (GameplayEffects|MakeOutgoingSpec (Ability|GetAbilitySystemComponent _ascharacter_base) "/Game/GameplayAbilitySystem/GameplayEffects/Character/Buffs/GE_HealFromLifesteal.GE_HealFromLifesteal_C" 1.0 (GameplayEffects|MakeEffectContext (Ability|GetAbilitySystemComponent _ascharacter_base))) "(TagName=\"Data.Damage\")" (* (.ReturnValue (Ability|Attribute|GetFloatAttributefromAbilitySystemComponent (Ability|GetAbilitySystemComponent _ascharacter_base) "(Attribute=\"/Script/Gunslinger.BaseAttributeSet:AttackPower\")")) (.ReturnValue (Ability|Attribute|GetFloatAttributefromAbilitySystemComponent (Ability|GetAbilitySystemComponent _ascharacter_base) "(Attribute=\"/Script/Gunslinger.BaseAttributeSet:LifeSteal\")")) -1.0)))
  (GameplayEffects|ApplyGameplayEffectSpecToSelf (Ability|GetAbilitySystemComponent _ascharacter_base) _returnvalue))

(event EventPostLogin
  (params (NewPlayer :type Player%20Controller%20Object%20Reference))
  (EventDispatchers|BindEventtoOnCharacterDied (delegate Custom|OncharDied)))

(fn ConstructionScript)