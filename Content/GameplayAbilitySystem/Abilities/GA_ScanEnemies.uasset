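; Gameplay ability that scans around the avatar and locks onto the nearest other actor as its CurrentTarget if that actor is a CharacterBase.
; An instant radius target actor, sized by an ability-system attribute, supplies candidates, and a loop narrows BaseDistance to find the closest.
; It turns the controller to face that character and activates Targeted-tagged abilities on both the previous target and the new one.
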(event Ability|EventActivateAbility
  (bind _returnvalue (Ability|GetAvatarActorfromActorInfo))
  (bind _data (|WaitTargetData :ConfirmationType "Instant" :Class "/Script/GameplayAbilities.GameplayAbilityTargetActor_Radius" :Radius (.ReturnValue (Ability|Attribute|GetFloatAttributefromAbilitySystemComponent (Ability|GetAbilitySystemComponent (Ability|GetAvatarActorfromActorInfo)) "(Attribute=\"/Script/Gunslinger.BaseAttributeSet:Range\")")) :StartLocation (Class|GameplayAbility|MakeTargetLocationInfofromOwnerActor) :ReticleClass "/Script/GameplayAbilities.GameplayAbilityWorldReticle")
    (:ValidData
      (bind _ascharacter_base (Utilities|Casting|CastToCharacterBase _returnvalue))
      (Utilities|IsValid (Variables|/Script/Gunslinger.CharacterBase|GetCurrentTarget _ascharacter_base)
        (:Is%20Valid
          (Class|CharacterBase|ActivateAbilitieswithTags (Variables|/Script/Gunslinger.CharacterBase|GetCurrentTarget _ascharacter_base) "(GameplayTags=((TagName=\"Character.States.Targeted\")))" true))
        (:Is%20Not%20Valid
          _))
      (for _array_element (Ability|TargetData|GetAllActorsfromTargetData _data)
        (if (!= _array_element _returnvalue)
          (if (<= (Transformation|GetDistanceTo _array_element _returnvalue) (Variables|Default|GetBaseDistance))
            (Variables|Default|SetTempActor _array_element)
            (Variables|Default|SetBaseDistance (Transformation|GetDistanceTo _array_element _returnvalue)))))
      (bind _ascharacter_base_2 (Utilities|Casting|CastToCharacterBase (Variables|Default|GetTempActor))
        (:then
          (bind _ascharacter_base_3 (Utilities|Casting|CastToCharacterBase _returnvalue))
          (Pawn|SetControlRotation (Pawn|GetController _ascharacter_base_3) (Math|Rotator|FindLookatRotation (.Location (Math|Transform|BreakTransform (Class|AbilitySystemBlueprintLibrary|GetTargetDataOrigin _data))) (Transformation|GetActorLocation (Variables|Default|GetTempActor))))
          (Variables|/Script/Gunslinger.CharacterBase|SetCurrentTarget _ascharacter_base_3 _ascharacter_base_2)
          (Class|CharacterBase|ActivateAbilitieswithTags _ascharacter_base_2 "(GameplayTags=((TagName=\"Character.States.Targeted\")))" true))
        (:CastFailed
          (Development|PrintString "not a character")))
      (Ability|EndAbility))
    (:Cancelled
      (Ability|EndAbility))))

(event Ability|EventOnEndAbility
  (params (bWasCancelled :type Boolean)))